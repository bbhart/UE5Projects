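; BP_Block is a destructible block actor that shows progressive destruction on its material before removing itself.
; On BeginPlay it creates a dynamic material instance of M_Block on its static mesh.
; StartDestroy plays a timeline that drives the DestroyAmount scalar parameter and destroys the actor on finish.
; StopDestroy halts the timeline and resets the parameter to zero, so interrupted destruction starts over.
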(event `self.ReceiveBeginPlay`
  (bind _returnvalue (`PrimitiveComponent.CreateDynamicMaterialInstance` (`self.SM_Block`) 0 "/Game/Materials/M_Block.M_Block" "None"))
  (set `self.thisMI` _returnvalue))

(event `StartDestroy`
  (bind (_direction _destroyamount) (`Timeline|DestroyBlockTimeline` :!via `PlayFromStart` :!label _label)
    (:`Update`
      (`MaterialInstanceDynamic.SetScalarParameterValue` (`self.thisMI`) "DestroyAmount" _destroyamount))
    (:`Finished`
      (`self.K2_DestroyActor`))))

(event `StopDestroy`
  (`MaterialInstanceDynamic.SetScalarParameterValue` (`self.thisMI`) "DestroyAmount" 0.0)
  (goto _label :!via `Stop`))

(fn `UserConstructionScript`)